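; BP_Interrupteur is a clickable switch actor that controls a BP_Lamp_Wall.
; On BeginPlay it caches all BP_Lamp_Wall actors, but only ever drives the first one found.
; Each click cycles that lamp through on at very high intensity, full Red value, then off with Red reset, using the lamp's own Intensity and Red values as state.
; A failed initial cast prints a failure message.
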(event `self.ReceiveActorOnClicked`
  (params (ButtonPressed :type "Key Structure"))
  (bind _output (`|GetArrayItem` (stale `self.ReceiveBeginPlay` _outactors)))
  (bind _asbp_lamp_wall (cast `/Game/Blueprints/BP_Lamp_Wall` _output)
    (:`then`
      (if (== (`/Game/Blueprints/BP_Lamp_Wall.Intensity` _asbp_lamp_wall) 0)
        (set `/Game/Blueprints/BP_Lamp_Wall.Intensity` 500000000 _asbp_lamp_wall)
        (else
          (bind _asbp_lamp_wall_2 (cast `/Game/Blueprints/BP_Lamp_Wall` _asbp_lamp_wall))
          (if (== (`/Game/Blueprints/BP_Lamp_Wall.Red` _asbp_lamp_wall_2) 0)
            (bind _asbp_lamp_wall_3 (cast `/Game/Blueprints/BP_Lamp_Wall` _output))
            (set `/Game/Blueprints/BP_Lamp_Wall.Red` 255 _asbp_lamp_wall_3)
            (else
              (bind _asbp_lamp_wall_4 (cast `/Game/Blueprints/BP_Lamp_Wall` _output))
              (set `/Game/Blueprints/BP_Lamp_Wall.Intensity` 0 _asbp_lamp_wall_4)
              (set `/Game/Blueprints/BP_Lamp_Wall.Red` 0 _asbp_lamp_wall_4))))))
    (:`CastFailed`
      (`KismetSystemLibrary.PrintString` "FAIL"))))

(event `self.ReceiveBeginPlay`
  (bind _outactors (`GameplayStatics.GetAllActorsOfClass` "/Game/Blueprints/BP_Lamp_Wall.BP_Lamp_Wall_C")))

(fn `UserConstructionScript`)