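; BP_Porte is a proximity door that shows exit text while the player is nearby and closes itself when they leave.
; Tick checks player distance to toggle the text and IsPlayerNear, which gates the OpenDoor event.
; Opening plays Animation; closing plays it and flips playback direction.
; IsDoorOpen updates only after each Delay, so the closing calls repeat every tick meanwhile while the player stays away.
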(event `self.ReceiveTick`
  (params (DeltaSeconds :type "Float (single-precision)"))
  (bind _exittext (`self.ExitText`))
  (bind _animation (`self.Animation`))
  ;[1 1 1] Toggle message visibility
  (if (<= (`self.GetDistanceTo` (`GameplayStatics.GetPlayerPawn` 0)) 350.0)
    (`SceneComponent.SetVisibility` _exittext true false)
    (set `self.IsPlayerNear` true)
    (else
      (`SceneComponent.SetVisibility` _exittext false false :!label _label)
      (set `self.IsPlayerNear` false)
      (if (`self.IsDoorOpen`)
        (`MatineeActor.Play` _animation)
        (`MatineeActor.ChangePlaybackDirection` _animation)
        (`KismetSystemLibrary.Delay` 2.0)
        (set `self.IsDoorOpen` false)))))

(event `self.ReceiveBeginPlay`
  ;[1 1 1] Toggle message visibility
  (goto _label))

(event `OpenDoor`
  ;[1 1 1] Animation Door Open
  (if (and (`self.IsPlayerNear`) (not (`self.IsDoorOpen`)))
    (`MatineeActor.Play` (`self.Animation`))
    (`KismetSystemLibrary.Delay` 2.0)
    (set `self.IsDoorOpen` true)))

(fn `UserConstructionScript`)